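; Firebase manager Blueprint that exercises a Firebase plugin (FBP nodes) as a test bed with mostly hardcoded sample data.
; BeginPlay connects and prints the result, but its following Sequence triggers no operations.
; Separate events wrap email auth, Realtime Database and document create/read/update/delete, with callbacks that print results or are empty stubs.
; Calls to most events and the batch-write chain are unwired; BatchOperate and DownloadFile are empty.
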(event Custom|Create%20Auth
  ;[1 1 1] Auth
  (Class|FBPAuth|FBPCreateAccountwithEmailandPassword (Variables|Info|GetCreateAccountEmail) (Variables|정보|GetCreateAccountPassword) (delegate Custom|Auth%20Success) (delegate Custom|Auth%20Fail)))

(event Custom|Auth%20Success
  (params (FirebaseUser :type BP%20Firebase%20User%20Structure))
  ;[1 1 1] Auth
  (Development|PrintString (.uid FirebaseUser)))

(event Custom|Listen%20for%20Sign%20In
  (params (FirebaseUser :type BP%20Firebase%20User%20Structure))
  ;[1 1 1] Listen Log In Out
  (Development|PrintString (Utilities|String|Append (.email FirebaseUser) "님이 입장하셨습니다.") true true "(R=0.031145,G=0.000000,B=1.000000,A=1.000000)"))

(event Custom|Listen%20for%20Sign%20Out
  ;[1 1 1] Listen Log In Out
  (Development|PrintString "Someone Signed Out"))

(event Custom|Verify%20User
  ;[1 1 1] VerifyUser
  (Class|FBPAuth|FBPSendVerificationEmail (delegate Custom|Verification%20Email%20Sent) (delegate Custom|Fail%20to%20Send%20Verification%20Email)))

(event Custom|Verification%20Email%20Sent
  ;[1 1 1] VerifyUser
  (Development|PrintString "Verification Email Sent"))

(event Custom|Fail%20to%20Send%20Verification%20Email
  (params (ErrorMessage :type String))
  ;[1 1 1] VerifyUser
  (Development|PrintString ErrorMessage))

(event Custom|On%20Document%20Added
  (params (DocumentID :type String))
  ;[1 1 1] Add Document
  (Development|PrintString (Utilities|String|Append "Document ID: " DocumentID)))

(event Custom|On%20Fail%20to%20Add%20Document
  (params (ErrorMessage :type String))
  ;[1 1 1] Add Document
  (Development|PrintString ErrorMessage true true "(R=1.000000,G=0.000000,B=0.057999,A=1.000000)" 4.0))

(event Custom|Add%20Document
  ;[1 1 1] Add Document
  (bind _returnvalue (Class|FBPDataObject|FBPBeginWriteDocument))
  (bind _returnvalue_2 (Class|FBPDataObject|AddString "name" "Potree" _returnvalue))
  (bind _returnvalue_3 (Class|FBPDataObject|AddStringArray "hobbies" (Utilities|Array|MakeArray "Play the Guitar" "Hang out w/ Friends" "Baseball") _returnvalue_2))
  (Class|FBPFirestore|FBPAddDocument (Utilities|Array|MakeArray "Users" "Potree") _returnvalue_3 (delegate Custom|On%20Document%20Added) (delegate Custom|On%20Fail%20to%20Add%20Document)))

(event Custom|UpdateDocument
  ;[1 1 1] UpdateDocuments
  (bind _returnvalue (Class|FBPDataObject|FBPBeginWriteDocument))
  (bind _returnvalue_2 (Class|FBPDataObject|AddString "Building" "Yeojusamgyo" _returnvalue))
  (Class|FBPFirestore|FBPUpdateDocument (Utilities|Array|MakeArray "Users" "KBuy3VA83I5qeFb1EJ53") _returnvalue_2 (delegate Custom|On%20Document%20Updated) (delegate Custom|On%20Fail%20to%20Updated%20Document)))

(event Custom|On%20Document%20Updated
  (params (DocumentID :type String))
  ;[1 1 1] UpdateDocuments
)

(event Custom|Auth%20Fail
  (params (ErrorMessage :type String))
  ;[1 1 1] Auth
)

(event Custom|On%20Fail%20to%20Updated%20Document
  (params (ErrorMessage :type String))
  ;[1 1 1] UpdateDocuments
)

(event Custom|DeleteDocument
  ;[1 1 1] DeleteDocuments
  (Class|FBPFirestore|FBPDeleteDocument (Utilities|Array|MakeArray "Users" "aqSRnV9HTQVbWNSz16F9") (delegate Custom|Document%20Deleted) (delegate Custom|Fail%20to%20Delete%20Document)))

(event Custom|Document%20Deleted
  ;[1 1 1] DeleteDocuments
  (Development|PrintString "Data Deleted"))

(event Custom|Fail%20to%20Delete%20Document
  (params (ErrorMessage :type String))
  ;[1 1 1] DeleteDocuments
)

(event Custom|Get%20Document
  ;[1 1 1] Get Document
  (Class|FBPFirestore|FBPListentoDocument (Utilities|Array|MakeArray "Users" "Potree") (delegate Custom|GetDocument_Retrieved) (delegate Custom|GetDocument_Fail)))

(event Custom|GetDocument_Retrieved
  (params (DocumentId :type String) (DocumentSnapshot :type Document%20Snapshot%20Structure))
  ;[1 1 1] Get Document
  (bind _returnvalue (Class|FBPDataObject|GetString "name" DocumentSnapshot))
  (Development|PrintString _returnvalue true true "(R=0.000000,G=0.660000,B=1.000000,A=1.000000)" 1e+01))

(event Custom|GetDocument_Fail
  (params (ErrorMessage :type String))
  ;[1 1 1] Get Document
)

(event Custom|Batch%20Complete
  ;[1 1 1] Batch Operate
)

(event Custom|Batch%20Fail
  (params (ErrorMessage :type String))
  ;[1 1 1] Batch Operate
)

(event Custom|Add%20Data
  ;[1 1 1] RealtimeDB
  ;;[1 1 1] Realtime Add Data
  (bind _returnvalue (Class|FBPDataObject|FBPBeginWriteDocument))
  (bind _returnvalue_2 (Class|FBPDataObject|AddString "name" "Potree" _returnvalue))
  (bind _returnvalue_3 (Class|FBPDataObject|AddNumber "age" 21.0 _returnvalue_2))
  (Class|FBPRealtimeDatabase|FBPAddData (Utilities|Array|MakeArray "Users" "Potree") _returnvalue_3 (delegate Custom|Data%20Added) (delegate Custom|Data%20Add%20failed)))

(event Custom|Sign%20In
  ;[1 1 1] Sign In
  (Class|FBPAuth|FBPSigninwithEmailandPassword (Variables|Info|GetCreateAccountEmail) (Variables|정보|GetCreateAccountPassword) (delegate Custom|Sign%20In%20Success) (delegate Custom|Sign%20In%20Fail)))

(event Custom|Data%20Added
  (params (DataId :type String))
  ;[1 1 1] RealtimeDB
  ;;[1 1 1] Realtime Add Data
)

(event Custom|Data%20Add%20failed
  (params (ErrorMessage :type String))
  ;[1 1 1] RealtimeDB
  ;;[1 1 1] Realtime Add Data
)

(event Custom|Batch%20Operate
  ;[1 1 1] Batch Operate
)

(event Custom|Update%20Data
  ;[1 1 1] RealtimeDB
  ;;[1 1 1] Realtime Update Data
  (bind _returnvalue (Class|FBPDataObject|FBPBeginWriteDocument))
  (bind _returnvalue_2 (Class|FBPDataObject|AddString "bio" "첫 고객" _returnvalue))
  (bind _returnvalue_3 (Class|FBPDataObject|AddNumber "age" 25.0 _returnvalue_2))
  (Class|FBPRealtimeDatabase|FBPUpdateData (Utilities|Array|MakeArray "Users" "Potree") _returnvalue_3 (delegate Custom|Data%20Updated) (delegate Custom|Data%20Updated%20Failed)))

(event Custom|Data%20Updated
  (params (DataId :type String))
  ;[1 1 1] RealtimeDB
  ;;[1 1 1] Realtime Update Data
)

(event Custom|Data%20Updated%20Failed
  (params (ErrorMessage :type String))
  ;[1 1 1] RealtimeDB
  ;;[1 1 1] Realtime Update Data
)

(event Custom|Delete%20Data
  ;[1 1 1] RealtimeDB
  ;;[1 1 1] Realtime Delete Data
  (Class|FBPRealtimeDatabase|FBPDeleteData (Utilities|Array|MakeArray "Users" "Potree") (delegate Custom|Data%20Deleted) (delegate Custom|Data%20Delete%20Failed)))

(event Custom|Data%20Deleted
  ;[1 1 1] RealtimeDB
  ;;[1 1 1] Realtime Delete Data
)

(event Custom|Data%20Delete%20Failed
  (params (ErrorMessage :type String))
  ;[1 1 1] RealtimeDB
  ;;[1 1 1] Realtime Delete Data
  (Development|PrintString ErrorMessage true true "(R=1.000000,G=0.007021,B=0.000000,A=1.000000)"))

(event Custom|Get%20Data
  (params (DataPath :type Array%20of%20Strings))
  ;[1 1 1] RealtimeDB
  ;;[1 1 1] Realtime Get Data
  (Class|FBPRealtimeDatabase|FBPListentoValue DataPath (delegate Custom|Data%20Recieved) (delegate Custom|Data%20Recieve%20Failed)))

(event Custom|Sign%20In%20Success
  (params (FirebaseUser :type BP%20Firebase%20User%20Structure))
  ;[1 1 1] Sign In
  (Development|PrintString (Utilities|String|Append (.email FirebaseUser) "님 환영합니다.") true true "(R=1.000000,G=0.000000,B=0.928204,A=1.000000)"))

(event Custom|Data%20Recieved
  (params (DataSnapshot :type Document%20Snapshot%20Structure))
  ;[1 1 1] RealtimeDB
  ;;[1 1 1] Realtime Get Data
  (bind _returnvalue (Class|FBPDataObject|GetNumber "age" DataSnapshot))
  (Development|PrintString (Utilities|String|ToString(Float) _returnvalue)))

(event Custom|Data%20Recieve%20Failed
  (params (ErrorMessage :type String))
  ;[1 1 1] RealtimeDB
  ;;[1 1 1] Realtime Get Data
  (Development|PrintString ErrorMessage true true "(R=1.000000,G=0.000000,B=0.155583,A=1.000000)"))

(event Custom|DownloadFile)

(event Custom|Sign%20In%20Fail
  (params (ErrorMessage :type String))
  ;[1 1 1] Sign In
)

(event Custom|Reset%20Password
  ;[1 1 1] Reset Password
  (Class|FBPAuth|FBPSendPasswordResetEmail (Variables|Info|GetCreateAccountEmail) (delegate Custom|On%20Password%20Reset%20Email%20Sent) (delegate Custom|On%20Fail%20to%20Send%20Password%20Reset%20Email)))

(event Custom|On%20Password%20Reset%20Email%20Sent
  (params (Email :type String))
  ;[1 1 1] Reset Password
  (Development|PrintString (Utilities|String|Append "Password Reset Email Sent to: " Email)))

(event Custom|On%20Fail%20to%20Send%20Password%20Reset%20Email
  (params (ErrorMessage :type String))
  ;[1 1 1] Reset Password
  (Development|PrintString ErrorMessage))

(event Custom|Listen%20For%20Sign%20In%20Changes
  ;[1 1 1] Listen Log In Out
  (Class|FBPAuth|FBPListenforSigninChanges (delegate Custom|Listen%20for%20Sign%20In) (delegate Custom|Listen%20for%20Sign%20Out)))

(event EventBeginPlay
  (bind _returnvalue (Class|FBPApp|FBPConnecttoFirebase))
  (if _returnvalue
    (Development|PrintString "Firebase와 연결되었습니다." true true "(R=0.000000,G=1.000000,B=0.168349,A=1.000000)")
    (Utilities|FlowControl|Sequence)
    (else
      (Development|PrintString "Firebase와 연결이 실패하였습니다." true true "(R=1.000000,G=0.000000,B=0.006121,A=1.000000)"))))

(fn ConstructionScript)