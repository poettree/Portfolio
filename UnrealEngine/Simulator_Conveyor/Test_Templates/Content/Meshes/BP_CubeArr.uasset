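; BP_CubeArr is an Actor Blueprint that lays out a flat grid of cube instances.
; Its Construction Script, when MaxX is positive, runs nested X/Y loops that add InstancedCubeMesh instances at Scaling-spaced local positions with Z at zero.
; The X loop runs through MaxX inclusive while Y stops at MaxY - 1, giving one extra step along X.
; The Event Graph holds only disabled placeholder events.
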(event EventBeginPlay)

(event Collision|EventActorBeginOverlap
  (params (OtherActor :type Actor%20Object%20Reference)))

(event EventTick
  (params (DeltaSeconds :type Float%20%28single-precision%29)))

(fn ConstructionScript
  (bind _scaling (Variables|Default|GetScaling))
  (if (> (Variables|Default|GetMaxX) 0)
    (for _index (range 0 (Variables|Default|GetMaxX))
      (for _index_2 (range 0 (- (Variables|Default|GetMaxY) 1))
        (Components|InstancedStaticMesh|AddInstance (Variables|Default|GetInstancedCubeMesh) (Math|Transform|MakeTransform (Math|Vector|MakeVector (Math|Conversions|ToFloat(Integer) (* _index _scaling)) (Math|Conversions|ToFloat(Integer) (* _scaling _index_2)) 0.0) "0, 0, 0" "1.000000,1.000000,1.000000") false)))))