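; Pawn Blueprint whose location is driven remotely by a value stored in Firebase.
; On BeginPlay it reads the collection and document paths from the Character row of the DB_DBPath data table, connects to Firebase and registers a value listener.
; Each change converts the document's Loc string to a vector and moves the actor there, printing the string; listener failures print their error message.
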(event Custom|ChangedValue
  (params (DataSnapshot :type Document%20Snapshot%20Structure))
  (bind _returnvalue (Class|FBPDataObject|GetString "Loc" DataSnapshot))
  (Development|PrintString _returnvalue)
  (Transformation|SetActorTransform (Math|Transform|MakeTransform (.OutConvertedVector (Math|Conversions|ToVector(Float) _returnvalue)) "0, 0, 0" "1.000000,1.000000,1.000000")))

(event Custom|Failed%20to%20Change%20Value
  (params (ErrorMessage :type String))
  (Development|PrintString ErrorMessage))

(event EventBeginPlay
  (bind _returnvalue (Utilities|GetDataTableRow "/Game/DB/DB_DBPath.DB_DBPath" "Character")
    (:then
      (bind _returnvalue_2 (Class|FBPApp|FBPConnecttoFirebase))
      (if _returnvalue_2
        (Class|FBPRealtimeDatabase|FBPListentoValue (Utilities|Array|MakeArray (.collectionpath _returnvalue) (.documentpath _returnvalue)) (delegate Custom|ChangedValue) (delegate Custom|Failed%20to%20Change%20Value))))))

(fn ConstructionScript)