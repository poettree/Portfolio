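; BP_Box is a cardboard box on a conveyor whose movement is driven by sensor values in Firebase.
; On BeginPlay it connects to Firebase and listens to Sensor1 and Sensor2, re-fetching a sensor's data when its value changes.
; A true Sensor1 eases the box along the conveyor.
; A true Sensor2 triggers the piston push on the player controller's conveyor and slides the box sideways in two chained moves.
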(event Custom|CustomEvent
  (params (DataSnapshot :type Document%20Snapshot%20Structure))
  (Development|PrintString "ListenValue")
  (Class|FBPRealtimeDatabase|FBPGetData (Utilities|Array|MakeArray "Conveyors" "Sensors" "Sensor2") (delegate Custom|CustomEvent_2) (delegate Custom|CustomEvent_3)))

(event Custom|CustomEvent_1
  (params (ErrorMessage :type String))
  (Development|PrintString ErrorMessage))

(event Custom|Data%20Recieved
  (params (DataSnapshot :type Document%20Snapshot%20Structure))
  (bind _returnvalue (Class|FBPDataObject|GetBoolean "Value" DataSnapshot))
  (if _returnvalue
    (CallFunction|Step1)))

(event Custom|Failed%20to%20Recieve
  (params (ErrorMessage :type String))
  (Development|PrintString ErrorMessage))

(event Custom|Step1
  (Components|MoveComponentTo (Variables|Default|GetConveyors_Cardboard_box) "0.000000,-150.000000,0.000000" "0, 0, 0" true true 3.0 false))

(event Custom|Step2
  (bind _conveyors_cardboard_box (Variables|Default|GetConveyors_Cardboard_box))
  (Default|PistonPush (Variables|/Game/Control/BP_PlayerController.BP_PlayerController_C|GetBP_Conveyor (stale EventBeginPlay _asbp_player_controller)))
  (Components|MoveComponentTo _conveyors_cardboard_box "-20.000000,-150.000000,0.000000" "0, 0, 0" false true 0.3 false)
  (Components|MoveComponentTo _conveyors_cardboard_box "-200.000000,-150.000000,0.000000" "0, 0, 0" true false 3.0 false))

(event Custom|CustomEvent_2
  (params (DataSnapshot :type Document%20Snapshot%20Structure))
  (bind _returnvalue (Class|FBPDataObject|GetBoolean "Value" DataSnapshot))
  (if _returnvalue
    (CallFunction|Step2)))

(event Custom|CustomEvent_3
  (params (ErrorMessage :type String))
  (Development|PrintString ErrorMessage))

(event Custom|ChangedValue
  (params (DataSnapshot :type Document%20Snapshot%20Structure))
  (Development|PrintString "ListenValue")
  (Class|FBPRealtimeDatabase|FBPGetData (Utilities|Array|MakeArray "Conveyors" "Sensors" "Sensor1") (delegate Custom|Data%20Recieved) (delegate Custom|Failed%20to%20Recieve)))

(event Custom|Failed%20to%20Change%20Value
  (params (ErrorMessage :type String))
  (Development|PrintString ErrorMessage))

(event EventBeginPlay
  (bind _asbp_player_controller (Utilities|Casting|CastToBP_PlayerController (Game|GetPlayerController 0)))
  (bind _returnvalue (Class|FBPApp|FBPConnecttoFirebase))
  (if _returnvalue
    (Utilities|FlowControl|Sequence
      (:then_0
        (Class|FBPRealtimeDatabase|FBPListentoValue (Utilities|Array|MakeArray "Conveyors" "Sensors" "Sensor1" "Value") (delegate Custom|ChangedValue) (delegate Custom|Failed%20to%20Change%20Value)))
      (:then_1
        (Class|FBPRealtimeDatabase|FBPListentoValue (Utilities|Array|MakeArray "Conveyors" "Sensors" "Sensor2" "Value") (delegate Custom|CustomEvent) (delegate Custom|CustomEvent_1))))))

(fn ConstructionScript)